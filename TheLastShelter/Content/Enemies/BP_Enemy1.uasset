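; Tower-defense enemy tied to a spline path that stops on hitting a turret, Mega Turret or base and damages it every Tick.
; It destroys drained targets and resumes, or destroys itself at the path's end.
; Enemy overlaps adjust VelocidadAvance by BichosDelPath order on shared paths, or by temporary speed changes across paths; movement itself happens outside this graph.
; Health lives in the Y scale of VidaActual, shrunk by ReducirVida.
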(event OnComponentBeginOverlap(CapsuleComponent)
  (params (OverlappedComponent :type Primitive%20Component%20Object%20Reference) (OtherActor :type Actor%20Object%20Reference) (OtherComp :type Primitive%20Component%20Object%20Reference) (OtherBodyIndex :type Integer) (bFromSweep :type Boolean) (SweepResult :type Hit%20Result%20Structure%20%28by%20ref%29))
  (bind _self self)
  (bind _pathdemovimiento (Variables|Default|GetPathDeMovimiento _self))
  (bind _bichosdelpath (Variables|/Game/BP_Path_1.BP_Path_1_C|GetBichosDelPath _pathdemovimiento))
  ;[1 1 1] Busqueda de objetivos (torres) en el rango y comprobacion de validez
  (if (Actor|ActorHasTag OtherActor "Torre")
    (bind _asbp_torre_1 (Utilities|Casting|CastToBP_Torre1 OtherActor)
      (:then
        (Variables|Default|SetObjetivo _asbp_torre_1))
      (:CastFailed
        ;[1 1 1] En caso de que colisione con la Mega Torre
        (bind _asbp_mega_turret (Utilities|Casting|CastToBP_MegaTurret OtherActor)
          (:then
            (Variables|Default|SetObjetivo%20MT _asbp_mega_turret))
          (:CastFailed
            ;[1 1 1] En caso de que colisione con la Base
            (bind _asbp_base (Utilities|Casting|CastToBP_Base OtherActor))
            (Variables|Default|SetObjetivo%20Base _asbp_base)))))
    (Variables|Default|SetVelocidadAvance 0.0)
    (Variables|Default|SetColisionTorre true)
    (elif (Actor|ActorHasTag OtherActor "Enemy")
      (bind _returnvalue (CallFunction|ComprobarDiferencias OtherActor))
      (if _returnvalue
        (bind _returnvalue_2 (CallFunction|ComprobarPaths OtherActor))
        (if _returnvalue_2
          (Variables|Default|SetVelocidadAvance 0.0)
          (bind _asbp_enemy_1 (Utilities|Casting|CastToBP_Enemy1 OtherActor))
          (if (< (Utilities|Array|FindItem _bichosdelpath _self) (Utilities|Array|FindItem _bichosdelpath _asbp_enemy_1))
            (if (Variables|Default|GetColisionTorre)
              _
              (else
                (Variables|Default|SetVelocidadAvance 1.0)))
            (Variables|BP_Enemy1_C|SetVelocidadAvance _asbp_enemy_1 0.0))
          (else
            (bind _asbp_enemy_1_2 (Utilities|Casting|CastToBP_Enemy1 OtherActor))
            (Variables|BP_Enemy1_C|SetVelocidadAvance _asbp_enemy_1_2 2.0)
            (Variables|Default|SetVelocidadAvance self 1.0)
            (Utilities|Time|SetTimerbyFunctionName 0 "Reiniciar Movimiento" 1.0)))))))

(event OnComponentEndOverlap(CapsuleComponent)
  (params (OverlappedComponent :type Primitive%20Component%20Object%20Reference) (OtherActor :type Actor%20Object%20Reference) (OtherComp :type Primitive%20Component%20Object%20Reference) (OtherBodyIndex :type Integer))
  ;[1 1 1] Busqueda de objetivos (torres) en el rango y comprobacion de validez
  (if (Actor|ActorHasTag OtherActor "Enemy")
    (bind _returnvalue (CallFunction|ComprobarDiferencias OtherActor))
    (if _returnvalue
      (Utilities|Time|SetTimerbyFunctionName 0 "Reiniciar Movimiento" 0.1))
    (elif (Actor|ActorHasTag OtherActor "Torre")
      (Variables|Default|SetVelocidadAvance 1.0)
      (Variables|Default|SetColisionTorre false))))

(event Custom|Reiniciar%20Movimiento
  ;[1 1 1] Busqueda de objetivos (torres) en el rango y comprobacion de validez
  (Variables|Default|SetVelocidadAvance 1.0))

(event EventTick
  (params (DeltaSeconds :type Float%20%28single-precision%29))
  (bind _objetivo_mt (Variables|Default|GetObjetivo%20MT))
  (bind _objetivo (Variables|Default|GetObjetivo))
  (bind _objetivo_base (Variables|Default|GetObjetivo%20Base))
  ;[1 1 1] Proceso de orientacion: el enemigo se orienta para estar justo en frente del objetivo (Torre)
  (Utilities|IsValid (Variables|Default|GetObjetivo)
    (:Is%20Valid
      (if (> (.Y (Math|Vector|BreakVector (Variables|/Script/Engine.SceneComponent|GetRelativeScale3D (Variables|/Game/Turrets/BP_Torre1.BP_Torre1_C|GetVidaActual _objetivo)))) 0.0)
        (Default|ReducirVida _objetivo (Variables|Default|GetDañoAtaque))
        (else
          (Actor|DestroyActor _objetivo)
          (Variables|Default|SetVelocidadAvance 1.0)
          (if (>= (Variables|Default|GetCurrentDistanceSpline) (Spline|GetSplineLength (Variables|/Game/BP_Path_1.BP_Path_1_C|GetCamino (Variables|Default|GetPathDeMovimiento))))
            (Actor|DestroyActor)))))
    (:Is%20Not%20Valid
      ;[1 1 1] Proceso de orientacion: el enemigo se orienta para estar justo en frente del objetivo (Mega Torre)
      (Utilities|IsValid (Variables|Default|GetObjetivo%20MT)
        (:Is%20Valid
          (if (> (.Y (Math|Vector|BreakVector (Variables|/Script/Engine.SceneComponent|GetRelativeScale3D (Variables|/Game/Turrets/BP_MegaTurret.BP_MegaTurret_C|GetVidaActual _objetivo_mt)))) 0.0)
            (Default|ReducirVida _objetivo_mt (Variables|Default|GetDañoAtaque))
            (else
              (Actor|DestroyActor _objetivo_mt)
              (Variables|Default|SetVelocidadAvance 1.0)
              (if (>= (Variables|Default|GetCurrentDistanceSpline) (Spline|GetSplineLength (Variables|/Game/BP_Path_1.BP_Path_1_C|GetCamino (Variables|Default|GetPathDeMovimiento))))
                (Actor|DestroyActor)))))
        (:Is%20Not%20Valid
          ;[1 1 1] Proceso de orientacion: el enemigo se orienta para estar justo en frente del objetivo (Base)
          (Utilities|IsValid (Variables|Default|GetObjetivo%20Base)
            (:Is%20Valid
              (if (> (.Y (Math|Vector|BreakVector (Variables|/Script/Engine.SceneComponent|GetRelativeScale3D (Variables|/Game/Turrets/BP_Base.BP_Base_C|GetVidaActual _objetivo_base)))) 0.0)
                (Default|ReducirVida _objetivo_base (Variables|Default|GetDañoAtaque))
                (else
                  (Actor|DestroyActor _objetivo_base)
                  (Variables|Default|SetVelocidadAvance 1.0)
                  (if (>= (Variables|Default|GetCurrentDistanceSpline) (Spline|GetSplineLength (Variables|/Game/BP_Path_1.BP_Path_1_C|GetCamino (Variables|Default|GetPathDeMovimiento))))
                    (Actor|DestroyActor)))))))))))

(fn ConstructionScript)

(fn ReducirVida
  (params (Daño :type Float%20%28single-precision%29))
  (bind _vidaactual (Variables|Default|GetVidaActual))
  (bind _relativescale3d (Variables|/Script/Engine.SceneComponent|GetRelativeScale3D _vidaactual))
  (bind _relativelocation (Variables|/Script/Engine.SceneComponent|GetRelativeLocation _vidaactual))
  (bind (_x _y _z) (Math|Vector|BreakVector _relativescale3d))
  (bind (_x_2 _y_2 _z_2) (Math|Vector|BreakVector _relativelocation))
  (bind _returnvalue (- _y Daño))
  (Transformation|SetRelativeScale3D _vidaactual (Math|Vector|MakeVector _x _returnvalue _z))
  (Transformation|SetRelativeLocation _vidaactual (Math|Vector|MakeVector _x_2 (- _y_2 0.5) _z_2) false false)
  (Variables|Default|SetVidaBicho _returnvalue))

(fn ComprobarDiferencias
  (params (ActorColsion :type Actor%20Object%20Reference))
  (bind _asbp_enemy_1 (Utilities|Casting|CastToBP_Enemy1 ActorColsion))
  (return (!= self _asbp_enemy_1)))

(fn ComprobarPaths
  (params (Enemigo :type Actor%20Object%20Reference))
  (bind _asbp_enemy_1 (Utilities|Casting|CastToBP_Enemy1 Enemigo))
  (return (== (Variables|Default|GetPathDeMovimiento self) (Variables|BP_Enemy1_C|GetPathDeMovimiento _asbp_enemy_1))))