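; Laser ball projectile Blueprint that damages enemies on overlap and cleans itself up.
; On overlap with an actor tagged Enemy, it casts to BP_Enemy1 and reads the Y scale of VidaActual as remaining health.
; It calls ReducirVida with Daño while that scale is positive, otherwise destroys the enemy, then destroys itself.
; A timer set on BeginPlay targets an erase event to remove bullets that hit nothing.
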(event Custom|erase%20Bullet
  ;[1 1 1] Borrar las balas que no han impactado cada 2 segundos
  (Utilities|IsValid self
    (:Is%20Valid
      (Actor|DestroyActor))))

(event EventBeginPlay
  ;[1 1 1] Borrar las balas que no han impactado cada 2 segundos
  (Utilities|Time|SetTimerbyFunctionName self "erase Bullet" 5.0 true))

(event Collision|EventActorBeginOverlap
  (params (OtherActor :type Actor%20Object%20Reference))
  ;[1 1 1] Destruir la bala cuando choca contra un enemigo
  (if (Actor|ActorHasTag OtherActor "Enemy")
    (bind _asbp_enemy_1 (Utilities|Casting|CastToBP_Enemy1 OtherActor))
    (if (> (.Y (Math|Vector|BreakVector (Variables|/Script/Engine.SceneComponent|GetRelativeScale3D (Variables|/Game/Enemies/BP_Enemy1.BP_Enemy1_C|GetVidaActual _asbp_enemy_1)))) 0.0)
      (Default|ReducirVida _asbp_enemy_1 (Variables|Default|GetDaño))
      (else
        (Actor|DestroyActor _asbp_enemy_1)))
    (Actor|DestroyActor)))

(fn ConstructionScript)