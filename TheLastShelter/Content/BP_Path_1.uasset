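; BP_Path_1 is an enemy path actor that spawns BP_Enemy1 enemies and moves them along its Camino spline.
; A looping timer counts down EnemigosTipo1, spawning each enemy at the spline start, tracking it in BichosDelPath and assigning it this path.
; Tick advances each enemy's own spline distance by Speed times VelocidadAvance, divided (not multiplied) by DeltaSeconds, then applies the spline's location and rotation.
; Invalid entries are removed during that same loop.
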(event Custom|SpawnEnemy
  ;[1 1 1] El enemigo se spawnea al inicio del path y lo recorrerá de forma independiente a todos los demas enemigos. Cada path tiene sus enemigos de cada tipo y cada enemigo sabe a que path pertenece
  (bind _output_get (Variables|Default|SetEnemigosTipo1 (- (Variables|Default|GetEnemigosTipo1) 1)))
  (if (>= _output_get 0)
    (bind _returnvalue (Game|SpawnActorfromClass "/Game/Enemies/BP_Enemy1.BP_Enemy1_C" (Spline|GetTransformatSplinePoint (Variables|Default|GetCamino) 0 "World" false) "Undefined" 0 0))
    (Utilities|Array|Add (Variables|Default|GetBichosDelPath) _returnvalue)
    (Variables|/Game/Enemies/BP_Enemy1.BP_Enemy1_C|SetPathDeMovimiento _returnvalue self)))

(event EventBeginPlay
  ;[1 1 1] Cada 2 segundos se spawnea un enemigo
  (Utilities|Time|SetTimerbyFunctionName 0 "SpawnEnemy" 2.0 true))

(event EventTick
  (params (DeltaSeconds :type Float%20%28single-precision%29))
  ;[1 1 1] En cada frame se cambia la posicion local de cada enemigo dentro del path. Cada enemigo pertenece a uno y solo a un unico path
  (for _array_element (Variables|Default|GetBichosDelPath)
    (bind _asbp_enemy_1 (Utilities|Casting|CastToBP_Enemy1 _array_element))
    (Utilities|IsValid _asbp_enemy_1
      (:Is%20Valid
        (bind _output_get (Variables|Default|SetBichoActual _asbp_enemy_1))
        (bind _transformacion (CallFunction|AjustarLocalizacionBicho DeltaSeconds _output_get))
        (Transformation|SetWorldTransform (Variables|/Script/Engine.Actor|GetRootComponent _output_get) _transformacion false false))
      (:Is%20Not%20Valid
        (Utilities|Array|RemoveItem (Variables|Default|GetBichosDelPath) _asbp_enemy_1)))))

(fn ConstructionScript)

(fn AjustarLocalizacionBicho
  (params (DeltaSeconds :type Float%20%28single-precision%29) (BichoActual :type BP%20Enemy%201%20Object%20Reference))
  (bind _camino (Variables|Default|GetCamino))
  (bind _output_get (Variables|/Game/Enemies/BP_Enemy1.BP_Enemy1_C|SetCurrentDistanceSpline BichoActual (+ (/ (* (Variables|Default|GetSpeed) (Variables|/Game/Enemies/BP_Enemy1.BP_Enemy1_C|GetVelocidadAvance BichoActual)) DeltaSeconds) (Variables|/Game/Enemies/BP_Enemy1.BP_Enemy1_C|GetCurrentDistanceSpline BichoActual))))
  (return (Math|Transform|MakeTransform (Spline|GetLocationatDistanceAlongSpline _camino _output_get "World") (Spline|GetRotationatDistanceAlongSpline _camino _output_get "World"))))