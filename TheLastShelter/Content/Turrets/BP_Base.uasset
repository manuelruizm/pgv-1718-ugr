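; BP_Base is a turret-game Blueprint with a visual health bar, the VidaActual component, that shrinks when damage is applied.
; ReducirVida lowers the bar's relative Y scale by a fixed step and shifts its relative Y location by DañoAtaque.
; Only the offset follows the damage amount, and the function tracks no numeric health and has no zero check.
; The event graph and construction script are empty.
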(event EventBeginPlay)

(event Collision|EventActorBeginOverlap
  (params (OtherActor :type Actor%20Object%20Reference)))

(event EventTick
  (params (DeltaSeconds :type Float%20%28single-precision%29)))

(fn ConstructionScript)

(fn ReducirVida
  (params (Daño%20Ataque :type Float%20%28single-precision%29))
  (bind _vidaactual (Variables|Default|GetVidaActual))
  (bind _relativescale3d (Variables|/Script/Engine.SceneComponent|GetRelativeScale3D _vidaactual))
  (bind _relativelocation (Variables|/Script/Engine.SceneComponent|GetRelativeLocation _vidaactual))
  (bind (_x _y _z) (Math|Vector|BreakVector _relativescale3d))
  (bind (_x_2 _y_2 _z_2) (Math|Vector|BreakVector _relativelocation))
  (Transformation|SetRelativeScale3D _vidaactual (Math|Vector|MakeVector _x (- _y 0.01) _z))
  (Transformation|SetRelativeLocation _vidaactual (Math|Vector|MakeVector _x_2 (- _y_2 Daño%20Ataque) _z_2) false false))