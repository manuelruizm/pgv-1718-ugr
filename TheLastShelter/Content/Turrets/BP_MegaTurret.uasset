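; Automated turret that acquires pawns tagged Enemy within range and fires BP_laser_ball at them.
; A looping sphere-trace timer picks the target and opens a Tick gate that line-traces it, closing when that trace hits a non-enemy or out-of-range actor.
; Tick interpolates head yaw and sets elevator pitch from a ballistic-arc formula, firing on a cooldown with recoil when roughly aligned.
; ReducirVida shrinks and shifts the health bar on damage.
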(event Custom|scanForTargetTimer
  (bind _self self)
  (bind _elevator (Variables|Default|GetElevator))
  (bind _barrelhead (Variables|Default|GetBarrelHead))
  (bind _elevator_2 (Variables|Default|GetElevator))
  (bind _speed (Variables|Default|Getspeed))
  (bind _gravity (Variables|Default|Getgravity))
  (bind _returnvalue (Transformation|GetWorldRotation _barrelhead))
  (bind _returnvalue_2 (Transformation|GetWorldRotation _elevator))
  (bind _returnvalue_3 (Transformation|GetWorldRotation _elevator_2))
  ;[1 1 1] Busca dentro de su rango un peón etiquetado como enemigo y comprueba que sea válido
  (bind _outhit (Collision|SphereTraceForObjects (Transformation|GetWorldLocation (Variables|Default|GetBarrelHead)) (Transformation|GetActorLocation _self) (Variables|Default|GettraceMaxDist) (Utilities|Array|MakeArray "ObjectTypeQuery3") false (Utilities|Array|MakeArray _self) "None"))
  (Utilities|IsValid (.HitActor (Collision|BreakHitResult _outhit))
    (:Is%20Valid
      (if (Actor|ActorHasTag (.HitActor (Collision|BreakHitResult _outhit)) "Enemy")
        (Utilities|IsValid (Variables|Default|GetfocusedTarget)
          (:Is%20Valid
            ;[1 1 1] Traza una linea entre la torreta y el enemigo que ha localizado
            (Utilities|FlowControl|Gate true) ; enters at Open
          )
          (:Is%20Not%20Valid
            (Variables|Default|SetfocusedTarget (.HitActor (Collision|BreakHitResult _outhit)))
            (Utilities|FlowControl|Gate true) ; enters at Open
          ))))))

(event Custom|closeFiringGate
  (bind _elevator (Variables|Default|GetElevator))
  (bind _barrelhead (Variables|Default|GetBarrelHead))
  (bind _elevator_2 (Variables|Default|GetElevator))
  (bind _speed (Variables|Default|Getspeed))
  (bind _gravity (Variables|Default|Getgravity))
  (bind _returnvalue (Transformation|GetWorldRotation _barrelhead))
  (bind _returnvalue_2 (Transformation|GetWorldRotation _elevator))
  (bind _returnvalue_3 (Transformation|GetWorldRotation _elevator_2))
  ;[1 1 1] Busca dentro de su rango un peón etiquetado como enemigo y comprueba que sea válido
  (CallFunction|ResetTurretOrientation)
  ;[1 1 1] Traza una linea entre la torreta y el enemigo que ha localizado
  (Utilities|FlowControl|Gate true) ; enters at Close
)

(event EventBeginPlay
  ;[1 1 1] Cada 0.2 busca un objetivo
  (Utilities|Time|SetTimerbyFunctionName self "scanForTargetTimer" 0.2 true))

(event EventTick
  (params (DeltaSeconds :type Float%20%28single-precision%29))
  (bind _elevator (Variables|Default|GetElevator))
  (bind _barrelhead (Variables|Default|GetBarrelHead))
  (bind _elevator_2 (Variables|Default|GetElevator))
  (bind _speed (Variables|Default|Getspeed))
  (bind _gravity (Variables|Default|Getgravity))
  (bind _returnvalue (Transformation|GetWorldRotation _barrelhead))
  (bind _returnvalue_2 (Transformation|GetWorldRotation _elevator))
  (bind _returnvalue_3 (Transformation|GetWorldRotation _elevator_2))
  ;[1 1 1] Busca dentro de su rango un peón etiquetado como enemigo y comprueba que sea válido
  ;[1 1 1] Traza una linea entre la torreta y el enemigo que ha localizado
  (Utilities|FlowControl|Gate true
    (:Exit
      (Utilities|IsValid (Variables|Default|GetfocusedTarget)
        (:Is%20Valid
          (bind _outhit (Collision|LineTraceForObjects (Transformation|GetWorldLocation (Variables|Default|GetBarrelHead)) (Transformation|GetActorLocation (Variables|Default|GetfocusedTarget)) (Utilities|Array|MakeArray "ObjectTypeQuery3" "ObjectTypeQuery1") false 0 "None" true "(R=0.044715,G=0.051031,B=1.000000,A=1.000000)" "(R=0.000000,G=1.000000,B=0.000000,A=1.000000)" 0.5)) ; Poner Draw debug a NINGUNO para no dibujar la linea
          ;[1 1 1] Comprueba que el objetivo sigue siendo válido y orienta el cañon hacia él
          (Utilities|IsValid (.HitActor (Collision|BreakHitResult _outhit))
            (:Is%20Valid
              (if (Actor|ActorHasTag (.HitActor (Collision|BreakHitResult _outhit)) "Enemy")
                (if (<= (Transformation|GetDistanceTo (.HitActor (Collision|BreakHitResult _outhit)) self) (Variables|Default|GettraceMaxDist))
                  (Transformation|SetWorldRotation (Variables|Default|GetBarrelHead) (Math|Rotator|MakeRotator (.Roll (Math|Rotator|BreakRotator (Math|Interpolation|RInterpTo _returnvalue (Math|Rotator|FindLookatRotation (Transformation|GetWorldLocation _barrelhead) (Transformation|GetActorLocation (Variables|Default|GetfocusedTarget))) (Utilities|Time|GetWorldDeltaSeconds) (Variables|Default|GetrotationHeadSpeed)))) 0.0 (.Yaw (Math|Rotator|BreakRotator (Math|Interpolation|RInterpTo _returnvalue (Math|Rotator|FindLookatRotation (Transformation|GetWorldLocation _barrelhead) (Transformation|GetActorLocation (Variables|Default|GetfocusedTarget))) (Utilities|Time|GetWorldDeltaSeconds) (Variables|Default|GetrotationHeadSpeed))))) false false)
                  ;[1 1 1] Hace el ángulo positivo
                  (if (< (Class|KismetMathLibrary|DegAtan (/ (+ (Math|Float|Power _speed 2.0) (Math|Float|Sqrt (- (Math|Float|Power _speed 4.0) (* _gravity (+ (* _gravity (Math|Float|Power (Transformation|GetDistanceTo (.HitActor (Collision|BreakHitResult _outhit)) self) 2.0)) (* (* (.Z (Math|Vector|BreakVector (Transformation|GetActorLocation (.HitActor (Collision|BreakHitResult _outhit))))) (Math|Float|Power _speed 2.0)) 2.0)))))) (* _gravity (Transformation|GetDistanceTo (.HitActor (Collision|BreakHitResult _outhit)) self)))) 0.0)
                    ;[1 1 1] En caso de que el ángulo sea negativo
                    (bind _output_get (Variables|Default|SetrotationAngleSpeed (Class|KismetMathLibrary|DegAtan (/ (+ (Math|Float|Power _speed 2.0) (Math|Float|Sqrt (- (Math|Float|Power _speed 4.0) (* _gravity (+ (* _gravity (Math|Float|Power (Transformation|GetDistanceTo (.HitActor (Collision|BreakHitResult _outhit)) self) 2.0)) (* (* (.Z (Math|Vector|BreakVector (Transformation|GetActorLocation (.HitActor (Collision|BreakHitResult _outhit))))) (Math|Float|Power _speed 2.0)) 2.0)))))) (* _gravity (Transformation|GetDistanceTo (.HitActor (Collision|BreakHitResult _outhit)) self))))))
                    (Transformation|SetWorldRotation _elevator (Math|Rotator|MakeRotator (.Roll (Math|Rotator|BreakRotator (Math|Interpolation|RInterpTo (Transformation|GetWorldRotation _elevator) (Math|Rotator|MakeRotator (.roll _returnvalue_2) (* _output_get -1.0) (.yaw _returnvalue_2)) (Utilities|Time|GetWorldDeltaSeconds) (Variables|Default|GetrotationAngleSpeed)))) (Math|Float|ClampAngle (.Pitch (Math|Rotator|BreakRotator (Math|Interpolation|RInterpTo (Transformation|GetWorldRotation _elevator) (Math|Rotator|MakeRotator (.roll _returnvalue_2) (* _output_get -1.0) (.yaw _returnvalue_2)) (Utilities|Time|GetWorldDeltaSeconds) (Variables|Default|GetrotationAngleSpeed)))) 0.0 89.0) (.Yaw (Math|Rotator|BreakRotator (Math|Interpolation|RInterpTo (Transformation|GetWorldRotation _elevator) (Math|Rotator|MakeRotator (.roll _returnvalue_2) (* _output_get -1.0) (.yaw _returnvalue_2)) (Utilities|Time|GetWorldDeltaSeconds) (Variables|Default|GetrotationAngleSpeed))))) false false)
                    (else
                      ;[1 1 1] En caso de que el ángulo sea positivo
                      (bind _output_get_2 (Variables|Default|SetrotationAngleSpeed (Class|KismetMathLibrary|DegAtan (/ (+ (Math|Float|Power _speed 2.0) (Math|Float|Sqrt (- (Math|Float|Power _speed 4.0) (* _gravity (+ (* _gravity (Math|Float|Power (Transformation|GetDistanceTo (.HitActor (Collision|BreakHitResult _outhit)) self) 2.0)) (* (* (.Z (Math|Vector|BreakVector (Transformation|GetActorLocation (.HitActor (Collision|BreakHitResult _outhit))))) (Math|Float|Power _speed 2.0)) 2.0)))))) (* _gravity (Transformation|GetDistanceTo (.HitActor (Collision|BreakHitResult _outhit)) self))))))
                      (Transformation|SetWorldRotation _elevator_2 (Math|Rotator|MakeRotator (.Roll (Math|Rotator|BreakRotator (Math|Interpolation|RInterpTo (Transformation|GetWorldRotation _elevator_2) (Math|Rotator|MakeRotator (.roll _returnvalue_3) _output_get_2 (.yaw _returnvalue_3)) (Utilities|Time|GetWorldDeltaSeconds) (Variables|Default|GetrotationAngleSpeed)))) (Math|Float|ClampAngle (.Pitch (Math|Rotator|BreakRotator (Math|Interpolation|RInterpTo (Transformation|GetWorldRotation _elevator_2) (Math|Rotator|MakeRotator (.roll _returnvalue_3) _output_get_2 (.yaw _returnvalue_3)) (Utilities|Time|GetWorldDeltaSeconds) (Variables|Default|GetrotationAngleSpeed)))) 0.0 89.0) (.Yaw (Math|Rotator|BreakRotator (Math|Interpolation|RInterpTo (Transformation|GetWorldRotation _elevator_2) (Math|Rotator|MakeRotator (.roll _returnvalue_3) _output_get_2 (.yaw _returnvalue_3)) (Utilities|Time|GetWorldDeltaSeconds) (Variables|Default|GetrotationAngleSpeed))))) false false)))
                  ;[1 1 1] Comprueba que el objetivo es válido y dispara en caso afirmativo
                  (if (Math|Rotator|Equal(Rotator) _returnvalue (Math|Rotator|FindLookatRotation (Transformation|GetWorldLocation _barrelhead) (Transformation|GetActorLocation (Variables|Default|GetfocusedTarget))) 22.0)
                    (Utilities|IsValid (.HitActor (Collision|BreakHitResult _outhit))
                      (:Is%20Valid
                        (CallFunction|ProjectileSpawner))
                      (:Is%20Not%20Valid
                        (Variables|Default|SetfocusedTarget 0))))
                  (else
                    (Variables|Default|SetfocusedTarget 0 :!label _label)
                    (CallFunction|CloseFiringGate)))
                (else
                  (goto _label))))))))))

(fn ConstructionScript)

(fn ResetTurretOrientation
  (bind _barrelhead (Variables|Default|GetBarrelHead))
  (Transformation|SetWorldRotation _barrelhead (Transformation|GetWorldRotation _barrelhead) false false)
  (return))

(fn ProjectileSpawner
  (bind _returnvalue (Utilities|Time|GetGameTimeinSeconds))
  ;[1 1 1] Comprueba el tiempo para ver si puede disparar y  hace que se cree la bala
  (if (> _returnvalue (Variables|Default|GetgameTimeFire))
    (Variables|Default|SetgameTimeFire (+ _returnvalue (Variables|Default|GetfireDelay)))
    (Game|SpawnActorfromClass "/Game/Bullets/BP_laser_ball.BP_laser_ball_C" (Transformation|GetWorldTransform (Variables|Default|GetSpawner%20Point)) "Undefined" 0 0)
    ;[1 1 1] Retroceso del cañón
    (Transformation|AddRelativeLocation (Variables|Default|GetBarrel) (Math|Vector|MakeVector (* (Variables|Default|GetbarrelRecoil) (Math|Conversions|ToFloat(Integer) (Variables|Default|Getalpha))) 0.0 0.0) false false)
    (Variables|Default|Setalpha (Math|Float|Truncate (* (Math|Conversions|ToFloat(Integer) (Variables|Default|Getalpha)) -1.0)))
    (Audio|PlaySound2D "/Game/Sounds/laserCannonShot_Cue.laserCannonShot_Cue")))

(fn ReducirVida
  (params (DañoAtaque :type Float%20%28single-precision%29))
  (bind _vidaactual (Variables|Default|GetVidaActual))
  (bind _relativescale3d (Variables|/Script/Engine.SceneComponent|GetRelativeScale3D _vidaactual))
  (bind _relativelocation (Variables|/Script/Engine.SceneComponent|GetRelativeLocation _vidaactual))
  (bind (_x _y _z) (Math|Vector|BreakVector _relativescale3d))
  (bind (_x_2 _y_2 _z_2) (Math|Vector|BreakVector _relativelocation))
  (Transformation|SetRelativeScale3D _vidaactual (Math|Vector|MakeVector _x (- _y 0.01) _z))
  (Transformation|SetRelativeLocation _vidaactual (Math|Vector|MakeVector _x_2 (- _y_2 DañoAtaque) _z_2) false false))