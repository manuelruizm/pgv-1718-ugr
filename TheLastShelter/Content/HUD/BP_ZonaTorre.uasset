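; Tower placement zone that spawns a basic tower or a mega turret when clicked while free and in edit mode.
; Toggling selectability swaps the zone's material to highlight free spots, and Torre1/Torre2 set the tower type to build.
; Placement marks the zone occupied and lowers energy through the HUD reference of Initializer actors tagged "Inicio".
; Tick frees the zone again once neither tower reference is valid.
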(event OnClicked(Zona)
  (params (TouchedComponent :type Primitive%20Component%20Object%20Reference) (ButtonPressed :type Key%20Structure))
  (bind _zona (Variables|Default|GetZona))
  (bind _returnvalue (Transformation|GetWorldLocation _zona))
  (bind _returnvalue_2 (Math|Conversions|ToTransform(Vector) _returnvalue))
  ;[1 1 1] Si está en modo edición (seleccionable) y se hace click sobre una zona libre (visible) ...
  (if (and (Variables|Default|GetVisible) (Variables|Default|GetSeleccionable))
    (Rendering|Material|SetMaterial (Variables|Default|GetZona) 0 "/Game/Materiales/EBase.EBase")
    ;[1 1 1] ... Dependiendo del tipo de torre elegida ...
    (if (Variables|Default|GetTipoTorre)
      ;[1 1 1] ... si es torre de tipo 1 se spawnea en la posición de la zona
      (bind _returnvalue_3 (Game|SpawnActorfromClass "/Game/Turrets/BP_Torre1.BP_Torre1_C" (Math|Conversions|ToTransform(Vector) (Transformation|GetWorldLocation (Variables|Default|GetZona))) "Undefined" 0 0))
      (Variables|Default|SetTorreBasica _returnvalue_3)
      (else
        ;[1 1 1] ... si es torre de tipo 2 se spawnea en la posición de la zona y con la Scale de la torre
        (bind _returnvalue_4 (Game|SpawnActorfromClass "/Game/Turrets/BP_MegaTurret.BP_MegaTurret_C" (Math|Transform|MakeTransform (.location _returnvalue_2) (.rotation _returnvalue_2) "1.500000,1.500000,0.250000") "Undefined" 0 0))
        (Variables|Default|SetMegaTorre _returnvalue_4)))
    (Variables|Default|SetVisible false)
    (bind _outactors (Actor|GetAllActorswithTag "Inicio"))
    (for _array_element _outactors
      (bind _asinitializer (Utilities|Casting|CastToInitializer _array_element))
      ;[1 1 1] Reducir la energía según el tipo de torre colocada
      (Default|BajarEnergía (Variables|/Game/Initializer.Initializer_C|GetHUD%20Reference _asinitializer) (Variables|Default|GetTipoTorre)))))

(event EventTick
  (params (DeltaSeconds :type Float%20%28single-precision%29))
  (Utilities|IsValid (Variables|Default|GetTorreBasica)
    (:Is%20Not%20Valid
      (Utilities|IsValid (Variables|Default|GetMegaTorre)
        (:Is%20Not%20Valid
          (Variables|Default|SetVisible true))))))

(fn ConstructionScript)

(fn CambiarVisibilidad
  ;[1 1 1] La visibilidad de la "zona torre" se refiere a cuando esa zona está libre (visible) u ocupada (no visible) por una torre.
  (Variables|Default|SetVisible (not (Variables|Default|GetVisible))))

(fn CambiarSeleccionabilidad
  ;[1 1 1] Entrar al modo edición para poder colocar una torre en una zona disponible
  (if (Variables|Default|GetSeleccionable)
    (Variables|Default|SetSeleccionable false)
    (Rendering|Material|SetMaterial (Variables|Default|GetZona) 0 0)
    (else
      ;[1 1 1] Si la zona está ocupada por otra torre, no se permite editar sobre ella
      (if (and (not (Variables|Default|GetSeleccionable)) (Variables|Default|GetVisible))
        (Variables|Default|SetSeleccionable (and (not (Variables|Default|GetSeleccionable)) (Variables|Default|GetVisible)))
        (Rendering|Material|SetMaterial (Variables|Default|GetZona) 0 "/Game/Materiales/EOrange.EOrange")))))

(fn Torre1
  (Variables|Default|SetTipoTorre true))

(fn Torre2
  (Variables|Default|SetTipoTorre false))